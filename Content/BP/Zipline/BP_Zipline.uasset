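; Zipline actor that links a start and end point with a cable and offers rides between them.
; InitCable runs on construction and BeginPlay, moving the cable to the start top and attaching its end to the end top.
; Colliders at each end send SetZiplineMessage to overlapping actors with that direction's permission flag and travel positions, then disable it on exit.
; The ride movement itself is left to the receiving actor.
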(event `self.ReceiveBeginPlay`
  (`self.initCable`))

(event `self.startCollider.OnComponentBeginOverlap`
  (params (OverlappedComponent :type "PrimitiveComponent Object Reference") (OtherActor :type "Actor Object Reference") (OtherComp :type "PrimitiveComponent Object Reference") (OtherBodyIndex :type Integer) (bFromSweep :type Boolean) (SweepResult :type "HitResult Structure (by ref)"))
  (message `/Game/BP/Zipline/BPI_ZiplineRider.setZipline` OtherActor (`self.can_zipline_from_start_to_end`) (`SceneComponent.K2_GetComponentLocation` (`self.startTop`)) (`SceneComponent.K2_GetComponentLocation` (`self.endTop`))))

(event `self.startCollider.OnComponentEndOverlap`
  (params (OverlappedComponent :type "PrimitiveComponent Object Reference") (OtherActor :type "Actor Object Reference") (OtherComp :type "PrimitiveComponent Object Reference") (OtherBodyIndex :type Integer))
  (message `/Game/BP/Zipline/BPI_ZiplineRider.setZipline` OtherActor false (0.0 0.0 0.0) (0.0 0.0 0.0)))

(event `self.endCollider.OnComponentBeginOverlap`
  (params (OverlappedComponent :type "PrimitiveComponent Object Reference") (OtherActor :type "Actor Object Reference") (OtherComp :type "PrimitiveComponent Object Reference") (OtherBodyIndex :type Integer) (bFromSweep :type Boolean) (SweepResult :type "HitResult Structure (by ref)"))
  (message `/Game/BP/Zipline/BPI_ZiplineRider.setZipline` OtherActor (`self.can_zipline_from_end_to_start`) (`SceneComponent.K2_GetComponentLocation` (`self.endTop`)) (`SceneComponent.K2_GetComponentLocation` (`self.startTop`))))

(event `self.endCollider.OnComponentEndOverlap`
  (params (OverlappedComponent :type "PrimitiveComponent Object Reference") (OtherActor :type "Actor Object Reference") (OtherComp :type "PrimitiveComponent Object Reference") (OtherBodyIndex :type Integer))
  (message `/Game/BP/Zipline/BPI_ZiplineRider.setZipline` OtherActor false (0.0 0.0 0.0) (0.0 0.0 0.0)))

(fn `UserConstructionScript`
  (`self.initCable`))